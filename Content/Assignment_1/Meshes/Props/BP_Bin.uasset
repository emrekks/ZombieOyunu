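; BP_Bin is a bin prop whose lid and bag meshes are varied at construction time, with no active gameplay logic.
; The Construction Script uses the Randomness flag to choose between the Random and Manuel (manual) functions.
; Random uses unseeded chance rolls to remove, open or close the lid.
; Manuel sets the lid from RemoveLid and LidOpen, and only it handles Tipped, which swaps the bag mesh.
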(event EventBeginPlay)

(event Collision|EventActorBeginOverlap
  (params (OtherActor :type Actor%20Object%20Reference)))

(event EventTick
  (params (DeltaSeconds :type Float%20%28single-precision%29)))

(fn ConstructionScript
  (if (Variables|Default|GetRandomness)
    (CallFunction|Random)
    (else
      (CallFunction|Manuel))))

(fn Random
  (bind _sm_binlid (Variables|Default|GetSM_BinLid))
  ;[1 1 1] Remove Lid
  (if (> (Math|Random|RandomFloatinRange 0.0 1.0) 0.75)
    (Components|DestroyComponent (Variables|Default|GetSM_BinLid))
    (else
      ;[1 1 1] Lid Open?
      (if (> (Math|Random|RandomFloatinRange 0.0 1.0) 0.75)
        (Transformation|SetRelativeRotation _sm_binlid (Math|Rotator|MakeRotator 0.0 9e+01 0.0) false false)
        (else
          (Transformation|SetRelativeRotation _sm_binlid (Math|Rotator|MakeRotator 0.0 0.0 0.0) false false))))))

(fn Manuel
  (bind _sm_binlid (Variables|Default|GetSM_BinLid))
  ;[1 1 1] Remove Lid
  (if (Variables|Default|GetRemove%20Lid)
    (Components|DestroyComponent (Variables|Default|GetSM_BinLid))
    (else
      ;[1 1 1] Lid Open?
      (if (Variables|Default|GetLid%20Open)
        (Transformation|SetRelativeRotation _sm_binlid (Math|Rotator|MakeRotator 0.0 9e+01 0.0) false false)
        (else
          (Transformation|SetRelativeRotation _sm_binlid (Math|Rotator|MakeRotator 0.0 0.0 0.0) false false)))))
  (if (Variables|Default|GetTipped)
    (Components|StaticMesh|SetStaticMesh (Variables|Default|GetSM_BinBag) "/Game/Assignment_1/Meshes/Props/Bin/SM_BinBag_2.SM_BinBag_2")))