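; BP_Locker_2 is a locker prop that varies its paint and door state in the construction script.
; ChoosePaint gives the body and the door each an independently random material from the first two PaintSelect entries.
; If RandomDoors is set, the door is either randomly removed (about a quarter of the time) or swung to a random yaw up to a right angle.
; Otherwise, RemoveDoor1 and LockerDoor1Rot control the door manually.
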(fn ConstructionScript
  (CallFunction|ChoosePaint)
  (if (Variables|Default|GetRandom%20Doors)
    (CallFunction|AutomaticDoors)
    (else
      (CallFunction|ManuelDoors))))

(fn AutomaticDoors
  (if (> (Math|Random|RandomFloatinRange 0.0 1.0) 0.75)
    (Components|DestroyComponent (Variables|Default|GetSM_LockerDoor_1))
    (else
      (Transformation|SetRelativeRotation (Variables|Default|GetSM_LockerDoor_1) (Math|Rotator|MakeRotator 0.0 0.0 (Math|Random|RandomFloatinRange 0.0 9e+01)) false false))))

(fn ManuelDoors
  (if (Variables|Default|GetRemove%20Door%201)
    (Components|DestroyComponent (Variables|Default|GetSM_LockerDoor_1))
    (else
      (Transformation|SetRelativeRotation (Variables|Default|GetSM_LockerDoor_1) (Math|Rotator|MakeRotator 0.0 0.0 (Variables|Default|GetLocker_Door_1%20Rot%20)) false false))))

(fn ChoosePaint
  (Rendering|Material|SetMaterial (Variables|Default|GetSM_Locker_1) 0 (Utilities|Array|Get(acopy) (Variables|Default|GetPaint%20Select) (Math|Random|RandomIntegerinRange 0 1)))
  (Rendering|Material|SetMaterial (Variables|Default|GetSM_LockerDoor_1) 0 (Utilities|Array|Get(acopy) (Variables|Default|GetPaint%20Select) (Math|Random|RandomIntegerinRange 0 1))))