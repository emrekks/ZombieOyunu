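; Ceiling light prop Blueprint that flickers on and off at random intervals from BeginPlay onward.
; The LightFlicker event waits on a retriggerable delay of random length, then a FlipFlop alternates between the off and on states.
; Each state sets the mesh's emissive material parameter and the rect light's intensity together, then the event calls itself to keep looping.
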(event Custom|Light%20Flicker
  (bind _sm_cieling_light (Variables|Default|GetSM_Cieling_Light))
  (bind _rectlight (Variables|Default|GetRectLight))
  (Utilities|FlowControl|RetriggerableDelay (Math|Random|RandomFloatinRange 0.25 2.5))
  (Utilities|FlowControl|FlipFlop
    (:A
      (Rendering|Material|SetScalarParameterValueonMaterials _sm_cieling_light "Emissive Multiply" 0.0)
      (Rendering|Components|Light|SetIntensity _rectlight 0.0))
    (:B
      (Rendering|Material|SetScalarParameterValueonMaterials _sm_cieling_light "Emissive Multiply" 75.0)
      (Rendering|Components|Light|SetIntensity _rectlight 8.0)))
  (CallFunction|LightFlicker))

(event EventBeginPlay
  (bind _sm_cieling_light (Variables|Default|GetSM_Cieling_Light))
  (bind _rectlight (Variables|Default|GetRectLight))
  (Utilities|FlowControl|RetriggerableDelay (Math|Random|RandomFloatinRange 0.25 2.5))
  (Utilities|FlowControl|FlipFlop
    (:A
      (Rendering|Material|SetScalarParameterValueonMaterials _sm_cieling_light "Emissive Multiply" 0.0)
      (Rendering|Components|Light|SetIntensity _rectlight 0.0))
    (:B
      (Rendering|Material|SetScalarParameterValueonMaterials _sm_cieling_light "Emissive Multiply" 75.0)
      (Rendering|Components|Light|SetIntensity _rectlight 8.0)))
  (CallFunction|LightFlicker))

(fn ConstructionScript)